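; Player Paper2D character that runs left and right, jumps, and swaps flipbook animations to match its movement.
; Axis input drives movement and, while not falling, picks an idle, run or fall state; jumping is allowed only when not falling.
; The state goes through a server event, and its RepNotify sets the sprite's flipbook and rotates it to face the run direction.
; The Jump state is handled there but never set here.
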(event `InputAxis|Move Right/left`
  (params (AxisValue :type "Float (single-precision)"))
  (`self.AddMovementInput` (`KismetMathLibrary.GetForwardVector` (`self.GetControlRotation`)) AxisValue)
  (if (`NavMovementComponent.IsFalling` (`self.CharacterMovement`))
    _
    (elif (== AxisValue 0.0)
      (if (> (.z (`self.GetVelocity`)) 0.0)
        (`self.SetMovementState` "NewEnumerator4")
        (else
          (`self.SetMovementState` "NewEnumerator0")))
      (elif (> AxisValue 0.0)
        (`self.SetMovementState` "NewEnumerator1")
        (else
          (`self.SetMovementState` "NewEnumerator2"))))))

(event `SetMovementState`
  (params (MovementState :type "/Game/blueprints/Enums/E_MovementState Enum" :default "NewEnumerator0"))
  (`self.SRV_SetMovementState` MovementState))

(event `SRV_SetMovementState`
  (params (`Movement State` :type "/Game/blueprints/Enums/E_MovementState Enum" :default "NewEnumerator0"))
  (set `self.MovementState` `Movement State`))

(event `InputAction|Jump`
  (params (Key :type "Key Structure"))
  (:`Pressed`
    (if (`self.IsnotJumping`)
      (`self.Jump`))))

(fn `IsnotJumping`
  (returns (ReturnValue :type Boolean))
  (return (not (`NavMovementComponent.IsFalling` (`self.CharacterMovement`)))))

(fn `OnRep_MovementState`
  (switch `/Game/blueprints/Enums/E_MovementState` (`self.MovementState`)
    (:`NewEnumerator0`
      (`PaperFlipbookComponent.SetFlipbook` (`self.Sprite`) "/Game/Assets/Characters/Mage/M_idle.M_idle"))
    (:`NewEnumerator1`
      (`SceneComponent.K2_SetRelativeRotation` :`self` (`self.Sprite`))
      (`PaperFlipbookComponent.SetFlipbook` (`self.Sprite`) "/Game/Assets/Characters/Mage/M_Run.M_Run"))
    (:`NewEnumerator2`
      (`SceneComponent.K2_SetRelativeRotation` (`self.Sprite`) (struct :`Yaw` 180.0) false true)
      (`PaperFlipbookComponent.SetFlipbook` (`self.Sprite`) "/Game/Assets/Characters/Mage/M_Run.M_Run"))
    (:`NewEnumerator3`
      (`PaperFlipbookComponent.SetFlipbook` (`self.Sprite`) "/Game/Assets/Characters/Serena/S_Jump.S_Jump"))
    (:`NewEnumerator4`
      (`PaperFlipbookComponent.SetFlipbook` (`self.Sprite`) "/Game/Assets/Characters/Serena/S_Jump.S_Jump"))))

(fn `UserConstructionScript`
  (`parent.UserConstructionScript`))